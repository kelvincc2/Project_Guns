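; TestProjectile is a projectile actor with a limited lifespan that damages EnemyDummy actors.
; Any collision box overlap applies damage if the actor is an EnemyDummy, then spawns a BulletHit effect facing the player and destroys the projectile.
; Calling the Cos event opens a gate on Tick, which then overrides local velocity to weave sideways along a cosine wave while moving forward.
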(event OnComponentBeginOverlap(CollisionBox)
  (params (OverlappedComponent :type Primitive%20Component%20Object%20Reference) (OtherActor :type Actor%20Object%20Reference) (OtherComp :type Primitive%20Component%20Object%20Reference) (OtherBodyIndex :type Integer) (bFromSweep :type Boolean) (SweepResult :type Hit%20Result%20Structure%20%28by%20ref%29))
  (bind _asenemy_dummy (Utilities|Casting|CastToEnemyDummy OtherActor)
    (:then
      (Game|Damage|ApplyDamage _asenemy_dummy 0.25 0 0))
    (:CastFailed
      _))
  (CallFunction|SpawnEmmiter)
  (Actor|DestroyActor))

(event Custom|Cos
  ;[1 1 1] Sine Example
  (Utilities|FlowControl|Gate true) ; enters at Open
)

(event EventBeginPlay
  (Actor|SetLifeSpan (Variables|Default|Getlifespan)))

(event EventTick
  (params (DeltaSeconds :type Float%20%28single-precision%29))
  ;[1 1 1] Sine Example
  (Utilities|FlowControl|Gate true
    (:Exit
      (Game|Components|ProjectileMovement|SetVelocityinLocalSpace (Variables|Default|GetProjectileMovement) (Math|Vector|MakeVector 1e+03 (* (Math|Trig|Cos(Radians) (* (Actor|GetGameTimeSinceCreation) 1e+01)) 1.5e+03) 0.0)))))

(fn ConstructionScript)

(fn SpawnEmmiter
  (bind _defaultsceneroot (Variables|Default|GetDefaultSceneRoot))
  (bind _returnvalue (Transformation|GetWorldLocation _defaultsceneroot))
  (Niagara|SpawnSystematLocation "/Game/VFX/Niagara/BulletHit.BulletHit" _returnvalue (Math|Rotator|FindLookatRotation _returnvalue (Transformation|GetWorldLocation (Variables|/Script/Engine.Character|GetCapsuleComponent (Game|GetPlayerCharacter 0))))))