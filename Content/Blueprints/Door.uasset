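; Door actor that swings open when a Character overlaps it, provided no actors of the MustBeGone class remain in the level.
; The OpenDoor timeline drives the door's yaw, with flags for 90 or 180 degrees and direction, and disables its collision.
; With DisplayQuest set, a QuestUI widget shows the class name and remaining count, polled every Tick, and is removed at zero.
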(event Collision|EventActorBeginOverlap
  (params (OtherActor :type Actor%20Object%20Reference))
  (bind _door (Variables|Default|GetDoor))
  (bind _returnvalue (Transformation|GetWorldRotation _door))
  (Utilities|Casting|CastToCharacter OtherActor)
  (bind _outactors (Actor|GetAllActorsOfClass (Variables|Default|GetMust%20be%20Gone)))
  (if (== (+ (Utilities|Array|LastIndex _outactors) 1) 0)
    (bind _open_door_90 (Timeline|Open%20Door Play)
      (:Update
        (Transformation|SetRelativeRotation _door (Math|Rotator|MakeRotator (.roll _returnvalue) (.pitch _returnvalue) (select (Variables|Default|GetOpening%20Direction) (* (select (Variables|Default|GetOpen%20180/90) (* _open_door_90 2.0) _open_door_90) -1.0) (select (Variables|Default|GetOpen%20180/90) (* _open_door_90 2.0) _open_door_90))) false false)
        (Collision|SetCollisionEnabled _door "NoCollision")))))

(event EventBeginPlay
  (if (Variables|Default|GetDisplayQuest)
    (bind _returnvalue (UserInterface|CreateWidget "/Game/Blueprints/UI/QuestUI.QuestUI_C"))
    (bind _output_get (Variables|Default|SetQuest%20UI%20REF _returnvalue))
    (UserInterface|Viewport|AddtoViewport _output_get 0)))

(event EventTick
  (params (DeltaSeconds :type Float%20%28single-precision%29))
  (bind _quest_ui_ref (Variables|Default|GetQuest%20UI%20REF))
  (if (Variables|Default|GetDisplayQuest)
    (Variables|/Game/Blueprints/UI/QuestUI.QuestUI_C|SetNameText _quest_ui_ref (Utilities|Text|ToText(String) (Utilities|GetClassDisplayName (Variables|Default|GetMust%20be%20Gone))))
    (Variables|/Game/Blueprints/UI/QuestUI.QuestUI_C|SetQuantityInt _quest_ui_ref (Variables|Default|GetQuantity))
    (bind _outactors (Actor|GetAllActorsOfClass (Variables|Default|GetMust%20be%20Gone)))
    (bind _output_get (Variables|Default|SetQuantity (+ (Utilities|Array|LastIndex _outactors) 1)))
    (if (<= _output_get 0)
      (Utilities|FlowControl|DoOnce false
        (:Completed
          (Widget|RemovefromParent (Variables|Default|GetQuest%20UI%20REF)))))))

(fn ConstructionScript)