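; PC_Main, apparently the main player controller, creates the main UI on begin play and handles pausing.
; Escape or Enter toggles pause by creating a pause widget and pausing the game, or removing it and resuming; an UnPause event shares the resume path.
; If the cursor was hidden, pausing shows it with Game and UI input focused on the widget, and a flag lets resuming hide it again.
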(event Custom|UnPause
  ;[1 1 1] Pause Mechanic
  (Widget|RemovefromParent (stale Input|KeyboardEvents|Enter _returnvalue_2))
  (Game|SetGamePaused false)
  (if (Variables|Default|GetMouseWasOff)
    (Variables|/Script/Engine.PlayerController|SetbShowMouseCursor (Game|GetPlayerController 0) false)
    (Variables|Default|SetMouseWasOff false)))

(event EventBeginPlay
  ;[1 1 1] Creating and adding to the main ui widget to the viewport
  (bind _returnvalue (UserInterface|CreateWidget "/Game/Blueprints/UI/MainUI.MainUI_C"))
  (UserInterface|Viewport|AddtoViewport _returnvalue 0))

(event Input|KeyboardEvents|Enter
  (params (Key :type Key%20Structure :default "None"))
  (bind _returnvalue (Game|GetPlayerController 0))
  ;[1 1 1] Pause Mechanic
  (:Pressed
    (if (Game|IsGamePaused)
      (Widget|RemovefromParent (stale _returnvalue_2))
      (Game|SetGamePaused false)
      (if (Variables|Default|GetMouseWasOff)
        (Variables|/Script/Engine.PlayerController|SetbShowMouseCursor _returnvalue false)
        (Variables|Default|SetMouseWasOff false))
      (else
        (bind _returnvalue_2 (UserInterface|CreateWidget "/Game/Blueprints/UI/PauseUI.PauseUI_C"))
        (UserInterface|Viewport|AddtoViewport _returnvalue_2 0)
        (Game|SetGamePaused true)
        (if (not (Variables|/Script/Engine.PlayerController|GetbShowMouseCursor _returnvalue))
          (bind _output_get (Variables|/Script/Engine.PlayerController|SetbShowMouseCursor _returnvalue true))
          (Variables|Default|SetMouseWasOff _output_get)
          (Input|SetInputModeGameandUI _returnvalue _returnvalue_2 "DoNotLock" false))))))

(event Input|KeyboardEvents|Escape
  (params (Key :type Key%20Structure :default "None"))
  (bind _returnvalue (Game|GetPlayerController 0))
  ;[1 1 1] Pause Mechanic
  (:Pressed
    (if (Game|IsGamePaused)
      (Widget|RemovefromParent (stale _returnvalue_2))
      (Game|SetGamePaused false)
      (if (Variables|Default|GetMouseWasOff)
        (Variables|/Script/Engine.PlayerController|SetbShowMouseCursor _returnvalue false)
        (Variables|Default|SetMouseWasOff false))
      (else
        (bind _returnvalue_2 (UserInterface|CreateWidget "/Game/Blueprints/UI/PauseUI.PauseUI_C"))
        (UserInterface|Viewport|AddtoViewport _returnvalue_2 0)
        (Game|SetGamePaused true)
        (if (not (Variables|/Script/Engine.PlayerController|GetbShowMouseCursor _returnvalue))
          (bind _output_get (Variables|/Script/Engine.PlayerController|SetbShowMouseCursor _returnvalue true))
          (Variables|Default|SetMouseWasOff _output_get)
          (Input|SetInputModeGameandUI _returnvalue _returnvalue_2 "DoNotLock" false))))))

(fn ConstructionScript)