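; EnemyDummy is a stationary-style enemy that turns toward the DemoCharacter and shoots at it while the player is inside its detection sphere.
; Sphere overlaps open and close a Tick gate that runs Shotting Mechanic, which spawns cooldown-limited projectiles, yaws the capsule and aims the muzzle, pitching only with CanShootY.
; Damage reduces normalized Health; at zero it stops attacking, enables mesh physics, drops capsule collision and destroys itself after a delay.
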(event OnComponentBeginOverlap(Sphere)
  (params (OverlappedComponent :type Primitive%20Component%20Object%20Reference) (OtherActor :type Actor%20Object%20Reference) (OtherComp :type Primitive%20Component%20Object%20Reference) (OtherBodyIndex :type Integer) (bFromSweep :type Boolean) (SweepResult :type Hit%20Result%20Structure%20%28by%20ref%29))
  (bind _asdemo_character (Utilities|Casting|CastToDemoCharacter OtherActor))
  (Utilities|FlowControl|Gate true) ; enters at Open
)

(event OnComponentEndOverlap(Sphere)
  (params (OverlappedComponent :type Primitive%20Component%20Object%20Reference) (OtherActor :type Actor%20Object%20Reference) (OtherComp :type Primitive%20Component%20Object%20Reference) (OtherBodyIndex :type Integer))
  (Utilities|Casting|CastToDemoCharacter OtherActor)
  (Utilities|FlowControl|Gate true) ; enters at Close
)

(event EventBeginPlay)

(event Collision|EventActorBeginOverlap
  (params (OtherActor :type Actor%20Object%20Reference)))

(event EventTick
  (params (DeltaSeconds :type Float%20%28single-precision%29))
  (if (not (Variables|Default|GetisDead?))
    (Utilities|FlowControl|Gate true
      (:Exit
        (|ShottingMechanic (stale OnComponentBeginOverlap(Sphere) _asdemo_character))))))

(event Game|Damage|EventAnyDamage
  (params (Damage :type Float%20%28single-precision%29) (DamageType :type Damage%20Type%20Object%20Reference) (InstigatedBy :type Controller%20Object%20Reference) (DamageCauser :type Actor%20Object%20Reference))
  ;[1 1 1] On enemy Take Damage
  (bind _output_get (Variables|Default|SetHealth (Math|Float|Clamp(Float) (- (Variables|Default|GetHealth) Damage))))
  (if (<= _output_get 0.0)
    (Variables|Default|SetisDead? true)
    (Physics|SetSimulatePhysics (Variables|Character|GetMesh) true)
    (Utilities|FlowControl|Delay 0.1)
    (Collision|SetCollisionEnabled (Variables|Collision|GetCapsuleComponent) "NoCollision")
    (Utilities|FlowControl|Delay 3.0)
    (Actor|DestroyActor)))

(fn ConstructionScript)