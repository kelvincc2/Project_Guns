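; Enemy projectile test actor that damages the DemoCharacter on overlap and has a short lifespan.
; Any overlap of its collision box spawns a BulletHit effect and destroys the projectile, with damage applied only to DemoCharacter.
; SpawnEmmiter orients the effect by a look-at rotation toward the negated velocity vector, used as a target position.
; An unwired sine example would weave the projectile via a cosine-driven local velocity, but Tick is empty.
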(event OnComponentBeginOverlap(CollisionBox)
  (params (OverlappedComponent :type Primitive%20Component%20Object%20Reference) (OtherActor :type Actor%20Object%20Reference) (OtherComp :type Primitive%20Component%20Object%20Reference) (OtherBodyIndex :type Integer) (bFromSweep :type Boolean) (SweepResult :type Hit%20Result%20Structure%20%28by%20ref%29))
  (bind _asdemo_character (Utilities|Casting|CastToDemoCharacter OtherActor)
    (:then
      (Game|Damage|ApplyDamage _asdemo_character 0.1 0 0))
    (:CastFailed
      _))
  (CallFunction|SpawnEmmiter)
  (Actor|DestroyActor))

(event EventBeginPlay
  (Actor|SetLifeSpan 4.0))

(event EventTick
  (params (DeltaSeconds :type Float%20%28single-precision%29))
  ;[1 1 1] Sine Example
)

(fn ConstructionScript)

(fn SpawnEmmiter
  (bind _defaultsceneroot (Variables|Default|GetDefaultSceneRoot))
  (bind _returnvalue (Transformation|GetWorldLocation _defaultsceneroot))
  (Niagara|SpawnSystematLocation "/Game/VFX/Niagara/BulletHit.BulletHit" _returnvalue (Math|Rotator|FindLookatRotation _returnvalue (* (Transformation|GetVelocity) -1))))